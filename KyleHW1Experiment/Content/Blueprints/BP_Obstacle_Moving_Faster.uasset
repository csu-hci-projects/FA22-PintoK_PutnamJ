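; BP_Obstacle_Moving_Faster is an obstacle actor that moves back and forth along a set direction.
; Tick offsets it each frame by the normalized Direction times ObstacleSpeed and delta time, without sweeping.
; A looping timer started on BeginPlay negates Direction every TimeToChange seconds to reverse the motion.
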(event Custom|ChangeDirection
  ;[1 1 1] Change Direction
  (Variables|Default|SetDirection (* (Variables|Default|GetDirection) -1.0)))

(event EventBeginPlay
  ;[1 1 1] Change Direction
  (Utilities|Time|SetTimerbyEvent (delegate Custom|ChangeDirection) (Variables|Default|GetTimeToChange) true))

(event Collision|EventActorBeginOverlap
  (params (OtherActor :type Actor%20Object%20Reference)))

(event EventTick
  (params (DeltaSeconds :type Float%20%28single-precision%29))
  ;[1 1 1] Every frame, update location
  (Transformation|AddActorWorldOffset (* (Math|Vector|Normalize (Variables|Default|GetDirection)) (* (Variables|Default|GetObstacleSpeed) (Utilities|Time|GetWorldDeltaSeconds)))))

(fn ConstructionScript)