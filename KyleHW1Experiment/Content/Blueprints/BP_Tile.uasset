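; BP_Tile is a floor tile that the player ball paints by touching it, counting toward an all-tiles-colored win.
; On first hit with paint remaining, it copies the ball's material, increments the controller's colored count and drains paint scaled by difficulty.
; When the count reaches the total, it calls AllTilesColored on PC_PlayerBall.
; Without paint, it briefly shows an insufficient-paint widget, guarded against stacking.
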(event EventBeginPlay)

(event Collision|EventActorBeginOverlap
  (params (OtherActor :type Actor%20Object%20Reference)))

(event EventTick
  (params (DeltaSeconds :type Float%20%28single-precision%29)))

(event Collision|EventHit
  (params (MyComp :type Primitive%20Component%20Object%20Reference) (Other :type Actor%20Object%20Reference) (OtherComp :type Primitive%20Component%20Object%20Reference) (bSelfMoved :type Boolean) (HitLocation :type Vector :default "0, 0, 0") (HitNormal :type Vector :default "0, 0, 0") (NormalImpulse :type Vector :default "0, 0, 0") (Hit :type Hit%20Result%20Structure%20%28by%20ref%29))
  ;[1 1 1] Convert Material to ball material on collision, increment tiles colored, remove some paint, check for win condition
  (if (not (Variables|Default|GetHasBeenTouched))
    (bind _asbp_player_ball (Utilities|Casting|CastToBP_PlayerBall Other))
    (bind _aspc_player_ball (Utilities|Casting|CastToPC_PlayerBall (Game|GetPlayerController 0)))
    (if (> (Variables|/Game/Blueprints/PC_PlayerBall.PC_PlayerBall_C|GetPaintRemaining _aspc_player_ball) 0.0001)
      (Rendering|Material|SetMaterial (Variables|Default|GetCube) 0 (Rendering|Material|GetMaterial (Variables|/Game/Blueprints/BP_PlayerBall.BP_PlayerBall_C|GetSphere _asbp_player_ball) 0))
      (bind _aspc_player_ball_2 (Utilities|Casting|CastToPC_PlayerBall (Game|GetPlayerController 0)))
      (bind _result (Math|Integer|IncrementInt (Variables|/Game/Blueprints/PC_PlayerBall.PC_PlayerBall_C|GetTilesColored _aspc_player_ball_2))
        (:%20%20
          (Variables|Default|SetHasBeenTouched true)
          (Variables|/Game/Blueprints/PC_PlayerBall.PC_PlayerBall_C|SetPaintRemaining _aspc_player_ball_2 (- (Variables|/Game/Blueprints/PC_PlayerBall.PC_PlayerBall_C|GetPaintRemaining _aspc_player_ball_2) (* (Variables|/Game/Blueprints/PC_PlayerBall.PC_PlayerBall_C|GetDifficultyLevel _aspc_player_ball_2) (Variables|/Game/Blueprints/PC_PlayerBall.PC_PlayerBall_C|GetDefaultPaintingDamage _aspc_player_ball_2))))
          (if (>= _result (Variables|/Game/Blueprints/PC_PlayerBall.PC_PlayerBall_C|GetTotalTiles _aspc_player_ball_2))
            (Default|AllTilesColored _aspc_player_ball_2))))
      (elif (not (Variables|Default|GetMessageDisplaying))
        (bind _returnvalue (UserInterface|CreateWidget "/Game/UI/InsufficientPaintMessage.InsufficientPaintMessage_C" _aspc_player_ball))
        (UserInterface|Viewport|AddtoViewport _returnvalue 0)
        (Variables|Default|SetMessageDisplaying true)
        (Utilities|FlowControl|Delay 1.0)
        (Variables|Default|SetMessageDisplaying false)
        (Widget|RemovefromParent _returnvalue)))))

(fn ConstructionScript)