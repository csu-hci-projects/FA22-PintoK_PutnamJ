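; Game mode for the ball game that starts the level through PC_PlayerBall on BeginPlay and provides menu and game-start functions.
; Main, level select and options menu functions each pause, show the cursor and add their widget.
; GetSaveDataFile locates a text save under Content/SaveData, creating it with defaults if missing.
; StartGame reads that file but opens Level0 regardless of content, then calls StartLevel.
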(event EventBeginPlay
  (bind _aspc_player_ball (Utilities|Casting|CastToPC_PlayerBall (Game|GetPlayerController 0)))
  (Default|StartLevel _aspc_player_ball))

(fn ConstructionScript)

(fn OpenMainMenu
  (Game|SetGamePaused true)
  (Variables|/Script/Engine.PlayerController|SetbShowMouseCursor (Game|GetPlayerController 0) true)
  (bind _returnvalue (UserInterface|CreateWidget "/Game/UI/MainMenu.MainMenu_C"))
  (UserInterface|Viewport|AddtoViewport _returnvalue 0))

(fn OpenLevelSelect
  (Game|SetGamePaused true)
  (Variables|/Script/Engine.PlayerController|SetbShowMouseCursor (Game|GetPlayerController 0) true)
  (bind _returnvalue (UserInterface|CreateWidget "/Game/UI/LevelSelectMenu.LevelSelectMenu_C"))
  (UserInterface|Viewport|AddtoViewport _returnvalue 0))

(fn OpenOptionsMenu
  (Game|SetGamePaused true)
  (Variables|/Script/Engine.PlayerController|SetbShowMouseCursor (Game|GetPlayerController 0) true)
  (bind _returnvalue (UserInterface|CreateWidget "/Game/UI/OptionsMenu.OptionsMenu_C"))
  (UserInterface|Viewport|AddtoViewport _returnvalue 0))

(fn StartGame
  (bind _filename (CallFunction|GetSaveDataFile))
  (bind (_lines _returnvalue) (Class|FileHelperBPLibrary|ReadLine _filename))
  (if _returnvalue
    (Game|OpenLevel(byObjectReference) "/Game/Maps/Level0.Level0" false)
    (else
      (Development|PrintString "Error when reading lines from save file! Opening default level..." true true "(R=1.000000,G=0.000000,B=0.000000,A=1.000000)" 5.0)
      (Game|OpenLevel(byObjectReference) "/Game/Maps/Level0.Level0" false)))
  (bind _aspc_player_ball (Utilities|Casting|CastToPC_PlayerBall (Game|GetPlayerController 0)))
  (Default|StartLevel _aspc_player_ball))

(fn GetSaveDataFile
  (bind _returnvalue (Class|BlueprintPathsLibrary|GetProjectFilePath))
  (bind _savefilename (Variables|Default|GetSaveFileName))
  (bind _returnvalue_2 (Utilities|String|FindSubstring _returnvalue "/" false true))
  (bind _returnvalue_3 (Utilities|String|ToString(Name) _savefilename))
  (bind _returnvalue_4 (Utilities|String|GetSubstring _returnvalue 0 _returnvalue_2))
  (bind _returnvalue_5 (Utilities|String|Append _returnvalue_4 "/Content/SaveData/"))
  (bind _returnvalue_6 (Utilities|String|Append _returnvalue_5 _returnvalue_3))
  (if true
    (bind _output_get (Variables|Default|SetSaveFileFullPathName _returnvalue_6))
    (bind _returnvalue_7 (Class|FileHelperBPLibrary|IsFile _output_get))
    (if _returnvalue_7
      (return (Variables|Default|GetSaveFileFullPathName))
      (else
        (Development|PrintString (Utilities|String|Append "File at location \"" _output_get "\" was not found. Creating it now."))
        (bind (_error _returnvalue_8) (Class|FileHelperBPLibrary|SaveLine (Variables|Default|GetSaveFileFullPathName) (Utilities|Array|MakeArray (Utilities|String|ToString(Text) (Class|KismetTextLibrary|AsTimeZoneDateTimeDateTime (Math|DateTime|Now) "MDT")) (Utilities|String|ToString(Name) (Variables|Default|GetLevel0)) (Utilities|String|ToString(Name) (Variables|Default|GetSelectedMaterialName)) (Utilities|String|ToString(Integer) 0)) true false))
        (if _returnvalue_8
          (Development|PrintString "Save File successfully created." true true "(R=0.000000,G=0.583333,B=0.000000,A=1.000000)")
          (return (Variables|Default|GetSaveFileFullPathName))
          (else
            (Development|PrintString (Utilities|String|Append "Error when writing default save file: " _error) true true "(R=1.000000,G=0.000000,B=0.000000,A=1.000000)" 5.0)))))
    (else
      (Development|PrintString (Utilities|String|Append "SaveFilePath file name could not be validated! Value: " _returnvalue_6) true true "(R=1.000000,G=0.000000,B=0.000000,A=1.000000)" 1e+01))))