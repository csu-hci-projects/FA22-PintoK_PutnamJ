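; Score pickup that spins in place and awards points when a BP_PlayerBall overlaps it.
; Tick applies a frame-rate-independent world rotation scaled by RotationSpeed, first nudging the rotation if it is near zero.
; On overlap it adds the default score amount multiplied by DifficultyLevel to CurrentScore on player 0's PC_PlayerBall controller, plays a sound at its location and destroys itself.
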(event EventTick
  (params (DeltaSeconds :type Float%20%28single-precision%29))
  ;[1 1 1] Float and Rotate
  (if (Utilities|Operators|EqualEqual :A (Transformation|GetActorRotation) :ErrorTolerance 0.01)
    (Transformation|SetActorRotation "0,1.000000, 0"))
  (Class|Actor|AddActorWorldRotation (* "0,1.000000,0" (* (Utilities|Time|GetWorldDeltaSeconds) (Variables|Default|GetRotationSpeed)))))

(event Collision|EventActorBeginOverlap
  (params (OtherActor :type Actor%20Object%20Reference))
  ;[1 1 1] On Pickup, add score, play sound, and destroy itself
  (Utilities|Casting|CastToBP_PlayerBall OtherActor)
  (bind _aspc_player_ball (Utilities|Casting|CastToPC_PlayerBall (Game|GetPlayerController 0)))
  (Variables|/Game/Blueprints/PC_PlayerBall.PC_PlayerBall_C|SetCurrentScore _aspc_player_ball (+ (Variables|/Game/Blueprints/PC_PlayerBall.PC_PlayerBall_C|GetCurrentScore _aspc_player_ball) (* (Variables|Default|GetDefaultScoreAmount) (Variables|/Game/Blueprints/PC_PlayerBall.PC_PlayerBall_C|GetDifficultyLevel _aspc_player_ball))))
  (Audio|PlaySoundatLocation "/Engine/EditorSounds/Notifications/CompileSuccess.CompileSuccess" (Transformation|GetActorLocation) "0, 0, 0" 0.5 1.0 0.0 0 0 0 0)
  (Actor|DestroyActor))

(fn ConstructionScript)