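; PaintSplatter is a reusable actor that briefly shows a paint splat beneath the player ball.
; On BeginPlay it registers itself with PC_PlayerBall so it can be reached through that controller.
; Its Spawn event copies the ball's material onto the Cylinder, teleports it just below the ball, plays a pop sound, then hides the actor again after a short delay.
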(event Custom|Spawn
  (bind _cylinder (Variables|Default|GetCylinder))
  ;[1 1 1] Show actor when called, then hide after a delay
  (bind _asbp_player_ball (Utilities|Casting|CastToBP_PlayerBall (Game|Player|GetPlayerPawn 0)))
  (Rendering|Material|SetMaterial (Variables|Default|GetCylinder) 0 (Rendering|Material|GetMaterial (Variables|/Game/Blueprints/BP_PlayerBall.BP_PlayerBall_C|GetSphere _asbp_player_ball) 0))
  (Transformation|SetWorldTransform (Variables|Default|GetCylinder) (Math|Transform|MakeTransform (Math|Vector|MakeVector (.X (Class|KismetMathLibrary|BreakVector3f (Transformation|GetWorldLocation (Variables|/Game/Blueprints/BP_PlayerBall.BP_PlayerBall_C|GetSphere _asbp_player_ball)))) (.Y (Class|KismetMathLibrary|BreakVector3f (Transformation|GetWorldLocation (Variables|/Game/Blueprints/BP_PlayerBall.BP_PlayerBall_C|GetSphere _asbp_player_ball)))) (- (.Z (Class|KismetMathLibrary|BreakVector3f (Transformation|GetWorldLocation (Variables|/Game/Blueprints/BP_PlayerBall.BP_PlayerBall_C|GetSphere _asbp_player_ball)))) 5e+01)) (Transformation|GetWorldRotation _cylinder) (Transformation|GetWorldScale _cylinder)) false true)
  (Rendering|SetActorHiddenInGame false)
  (Audio|PlaySound2D "/Game/Interface_And_Item_Sounds/WAV/Abstract_Pop_01.Abstract_Pop_01" 1.0 1.0 0.0 0 0)
  (Utilities|FlowControl|Delay 1.0)
  (Rendering|SetActorHiddenInGame true))

(event Collision|EventActorBeginOverlap
  (params (OtherActor :type Actor%20Object%20Reference)))

(event EventTick
  (params (DeltaSeconds :type Float%20%28single-precision%29)))

(event EventBeginPlay
  ;[1 1 1] Give the Player Controller a reference to self
  (bind _aspc_player_ball (Utilities|Casting|CastToPC_PlayerBall (Game|GetPlayerController 0)))
  (Variables|/Game/Blueprints/PC_PlayerBall.PC_PlayerBall_C|SetPaintSplatterRef _aspc_player_ball self))

(fn ConstructionScript)