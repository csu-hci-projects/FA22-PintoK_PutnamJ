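; Orange paint pickup that spins in the world and refills the player's paint when BP_PlayerBall overlaps it.
; Tick applies a frame-rate-independent yaw rotation at RotationSpeed.
; Overlap adds a restore amount divided by difficulty level to PC_PlayerBall's PaintRemaining, capped at full, and plays a fill sound.
; The pickup then hides and ignores overlaps for ten seconds before becoming collectable again.
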(event EventTick
  (params (DeltaSeconds :type Float%20%28single-precision%29))
  ;[1 1 1] Float and Rotate
  (if (Utilities|Operators|EqualEqual :A (Transformation|GetActorRotation) :ErrorTolerance 0.01)
    (Transformation|SetActorRotation "0,1.000000, 0"))
  (Class|Actor|AddActorWorldRotation (* "0,1.000000,0" (* (Utilities|Time|GetWorldDeltaSeconds) (Variables|Default|GetRotationSpeed)))))

(event Collision|EventActorBeginOverlap
  (params (OtherActor :type Actor%20Object%20Reference))
  ;[1 1 1] On Pickup, add paint, play sound, and hide for 10 seconds
  (if (not (Variables|Default|GetPickedUp))
    (Utilities|Casting|CastToBP_PlayerBall OtherActor)
    (bind _aspc_player_ball (Utilities|Casting|CastToPC_PlayerBall (Game|GetPlayerController 0)))
    (Variables|/Game/Blueprints/PC_PlayerBall.PC_PlayerBall_C|SetPaintRemaining _aspc_player_ball (Math|Float|Min(Float) (+ (Variables|/Game/Blueprints/PC_PlayerBall.PC_PlayerBall_C|GetPaintRemaining _aspc_player_ball) (/ (Variables|Default|GetDefaultPaintRestoreAmount) (Variables|/Game/Blueprints/PC_PlayerBall.PC_PlayerBall_C|GetDifficultyLevel _aspc_player_ball))) 1.0))
    (Audio|PlaySoundatLocation "/Game/Interface_And_Item_Sounds/WAV/Bar_Filling_01.Bar_Filling_01" (Transformation|GetActorLocation) "0, 0, 0" 0.25 1.0 0.0 0 0 0 0)
    (Rendering|SetActorHiddenInGame true)
    (Variables|Default|SetPickedUp true)
    (Utilities|FlowControl|Delay 1e+01)
    (Rendering|SetActorHiddenInGame false)
    (Variables|Default|SetPickedUp false)))

(fn ConstructionScript)