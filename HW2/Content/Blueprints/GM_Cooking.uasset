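; Cooking game mode that matches selected ingredients against five recipes and tracks discovered dishes in the Cookbook map.
; BeginCooking joins selected ingredient keys into an order-sensitive string, compares it to each joined recipe, then maps the index to a Cookbook key, so both orders must align.
; Sounds distinguish failed, repeat and new dishes, with sparks for new ones.
; CheckWinCondition fires GameIsWon once all are discovered, playing a fanfare and turning pot and lid gold.
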(event Custom|Start%20Sparks
  ;[1 1 1] Handle Spark Generation Effect
  (bind _returnvalue (Effects|SpawnEmitteratLocation "/Game/StarterContent/Particles/P_Sparks.P_Sparks" "150.000000,43.639999,100.000000" "0, 0, 0" "1.000000,1.000000,1.000000" false))
  (Utilities|FlowControl|Delay 1.5)
  (Components|DestroyComponent _returnvalue))

(event Custom|GameIsWon
  ;[1 1 1] Handle Game Win Events
  (Utilities|FlowControl|Delay 1.5)
  (Audio|PlaySound2D "/Game/Sounds/yt5s_io_-_Mario_Kart_Wii_-_Winner_Sound_320_kbps.yt5s_io_-_Mario_Kart_Wii_-_Winner_Sound_320_kbps" 0.2 1.0 0.0 0 0)
  (bind _returnvalue (Actor|GetActorOfClass "/Game/Blueprints/BP_CookingLid.BP_CookingLid_C"))
  (Rendering|Material|SetMaterial (Variables|/Game/Blueprints/BP_CookingLid.BP_CookingLid_C|GetCylinder _returnvalue) 0 "/Game/StarterContent/Materials/M_Metal_Gold.M_Metal_Gold")
  (bind _returnvalue_2 (Actor|GetActorOfClass "/Game/Blueprints/BP_CookingPot.BP_CookingPot_C"))
  (Rendering|Material|SetMaterial (Variables|/Game/Blueprints/BP_CookingPot.BP_CookingPot_C|GetPot _returnvalue_2) 0 "/Game/StarterContent/Materials/M_Metal_Gold.M_Metal_Gold"))

(event EventBeginPlay
  ;[1 1 1] Make sure the dish order here is the exact same as in the Recipes Struct!
  (bind _returnvalue (Actor|GetActorOfClass "/Game/Blueprints/BP_CookingLid.BP_CookingLid_C"))
  (Rendering|Material|SetMaterial (Variables|/Game/Blueprints/BP_CookingLid.BP_CookingLid_C|GetCylinder _returnvalue) 0 "/Game/Materials/M_Cauldron.M_Cauldron")
  (bind _returnvalue_2 (Actor|GetActorOfClass "/Game/Blueprints/BP_CookingPot.BP_CookingPot_C"))
  (Rendering|Material|SetMaterial (Variables|/Game/Blueprints/BP_CookingPot.BP_CookingPot_C|GetPot _returnvalue_2) 0 "/Game/Materials/M_Cauldron.M_Cauldron")
  (Variables|Default|SetCookbook (Utilities|Map|MakeMap (Utilities|String|ToString(Name) "Dish0") (Math|Conversions|ToBoolean(Integer) 0) "Dish1" false "Dish2" false "Dish3" false "Dish4" false))
  (Variables|Default|SetGameWin false))

(fn ConstructionScript)

(fn BeginCooking
  (params (CurrentIngredients :type Map%20of%20Strings%20to%20Booleans))
  (bind _recipes (Variables|Default|GetRecipes))
  (bind _cookbook (Variables|Default|GetCookbook))
  (bind (_dish0 _dish1 _dish2 _dish3 _dish4) (Utilities|Struct|BreakRecipes _recipes))
  (bind _keys (Utilities|Map|Keys CurrentIngredients))
  (bind _values (Utilities|Map|Values CurrentIngredients))
  (for (_array_element _array_index) _values
    (if _array_element
      (Utilities|Array|Add (Variables|Default|GetIngredientArray) (Utilities|Array|Get(acopy) _keys _array_index))))
  (bind (_array_element_2 _array_index_2) (Utilities|Array|ForEachLoopwithBreak (Utilities|Array|MakeArray (Utilities|String|JoinStringArray _dish0 "") (Utilities|String|JoinStringArray _dish1 "") (Utilities|String|JoinStringArray _dish2 "") (Utilities|String|JoinStringArray _dish3 "") (Utilities|String|JoinStringArray _dish4 "")) :!label _label)
    (:LoopBody
      (if (Utilities|Enum|Equal(Enum) (Utilities|String|JoinStringArray (Variables|Default|GetIngredientArray) "") _array_element_2)
        (bind _keys_2 (Utilities|Map|Keys (Variables|Default|GetCookbook)))
        (Variables|Default|SetCreatedDish (Utilities|Array|Get(acopy) _keys_2 _array_index_2))
        (goto _label Break)))
    (:Completed
      (Utilities|Array|Clear (Variables|Default|GetIngredientArray))
      (if (Utilities|Enum|Equal(Enum) (Variables|Default|GetCreatedDish) "")
        (Audio|PlaySound2D "/Engine/EditorSounds/Notifications/CompileFailed.CompileFailed" 0.5 1.0 0.0 0 0) ; Failure Dish
        (return)
        (else
          (if (.Value (Utilities|Map|Find _cookbook (Variables|Default|GetCreatedDish)))
            (Audio|PlaySound2D "/Engine/EditorSounds/GamePreview/EndSimulate.EndSimulate" 0.5 1.0 0.0 0 0) ; Dish Previously Created
            (else
              (Audio|PlaySound2D "/Engine/EditorSounds/GamePreview/StartPlayInEditor.StartPlayInEditor" 0.5 1.0 0.0 0 0) ; New Dish
              (CallFunction|StartSparks)
              (Utilities|Map|Add _cookbook (Variables|Default|GetCreatedDish) true)))
          (Variables|Default|SetCreatedDish "")
          (CallFunction|CheckWinCondition)
          (return))))))

(fn CheckWinCondition
  (if (Variables|Default|GetGameWin)
    (return)
    (else
      (bind _values (Utilities|Map|Values (Variables|Default|GetCookbook)))
      (bind _array_element (Utilities|Array|ForEachLoopwithBreak _values :!label _label)
        (:LoopBody
          (if _array_element
            (Variables|Default|SetGameWin true)
            (else
              (Variables|Default|SetGameWin false)
              (goto _label Break))))
        (:Completed
          (if (Variables|Default|GetGameWin)
            (CallFunction|GameIsWon)
            (return)
            (else
              (return))))))))