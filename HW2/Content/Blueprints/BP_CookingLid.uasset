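; BP_CookingLid is a grabbable lid for a cooking pot that moves between a starting spot and a closed position on the pot.
; Respawn, called on BeginPlay, teleports the cylinder component to its initial transform, while CloseLid teleports it to the pot's transform.
; Both functions unhide the actor, force-release the grab component and set a different grab type for each state.
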(event EventBeginPlay
  (CallFunction|Respawn))

(fn ConstructionScript)

(fn Respawn
  (bind _grabcomponent (Variables|Default|GetGrabComponent))
  (Transformation|SetWorldTransform (Variables|Default|GetCylinder) (Variables|Default|GetInitialLocation) false true)
  (Rendering|SetActorHiddenInGame false)
  (Default|TryRelease _grabcomponent)
  (Variables|/Game/VRTemplate/Blueprints/GrabComponent.GrabComponent_C|SetGrabType _grabcomponent "NewEnumerator4"))

(fn CloseLid
  (bind _grabcomponent (Variables|Default|GetGrabComponent))
  (Transformation|SetWorldTransform (Variables|Default|GetCylinder) (Variables|Default|GetCookingPotLocation) false true)
  (Rendering|SetActorHiddenInGame false)
  (Default|TryRelease _grabcomponent)
  (Variables|/Game/VRTemplate/Blueprints/GrabComponent.GrabComponent_C|SetGrabType _grabcomponent "NewEnumerator0"))