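; BP_Sink is a grabbable sink that empties the cooking pot.
; On grab, it finds BP_CookingPot by class and, unless the pot is cooking, plays a sound at the sink and clears the pot's current ingredients.
; It then releases the GrabComponent immediately, so the grab acts as a button press.
; A node resetting the Faucet's location is left unconnected.
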(event OnGrabbed(GrabComponent)
  (bind _returnvalue (Actor|GetActorOfClass "/Game/Blueprints/BP_CookingPot.BP_CookingPot_C"))
  (if (Variables|/Game/Blueprints/BP_CookingPot.BP_CookingPot_C|GetCurrentlyCooking _returnvalue)
    _
    (else
      (Audio|PlaySoundatLocation "/Engine/VREditor/Sounds/VR_open.VR_open" (Transformation|GetActorLocation) "0, 0, 0" 0.5 1.0 0.0 0 0 0 0)
      (Default|ClearCurrentIngredients _returnvalue)))
  (Default|TryRelease (Variables|Default|GetGrabComponent)))

(event EventBeginPlay)

(event Collision|EventActorBeginOverlap
  (params (OtherActor :type Actor%20Object%20Reference)))

(event EventTick
  (params (DeltaSeconds :type Float%20%28single-precision%29)))

(fn ConstructionScript)