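; Grabbable physics ingredient actor that can reset itself to a stored starting transform.
; BeginPlay and the ResetIngredientPosition event both run Respawn.
; Respawn zeroes the Cube's linear and angular velocity, teleports it to InitialLocation, unhides the actor and releases the GrabComponent's hold.
; InitialLocation is only read here, never captured in these graphs.
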(event Custom|Reset%20Ingredient%20Position
  (CallFunction|Respawn))

(event EventBeginPlay
  (CallFunction|Respawn))

(fn ConstructionScript)

(fn Respawn
  (Physics|SetPhysicsLinearVelocity (Variables|Default|GetCube) "0, 0, 0" false "None")
  (Class|PrimitiveComponent|SetPhysicsAngularVelocityinRadians (Variables|Default|GetCube) "0, 0, 0" false "None")
  (Transformation|SetWorldTransform (Variables|Default|GetCube) (Variables|Default|GetInitialLocation) false true)
  (Rendering|SetActorHiddenInGame false)
  (Default|TryRelease (Variables|Default|GetGrabComponent)))